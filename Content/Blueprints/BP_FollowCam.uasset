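; BP_FollowCam is a follow camera actor for a side-scroller that tracks BP_SideScrollerCharacter along the X axis.
; BeginPlay caches the cast player character as PlayerReference.
; Each Tick moves the actor to the player's X, with Y taken from an increment on Offset.Y and Z held at a hardcoded height.
; The construction script pre-positions it at the character's location plus the full Offset vector.
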(event `self.ReceiveBeginPlay`
  ;[0 1 0.03341 0.5] Store a Reference to Player
  (bind _asbp_side_scroller_character (cast `/Game/Blueprints/BP_SideScrollerCharacter` (`GameplayStatics.GetPlayerCharacter` 0)))
  (set `self.Player Reference` _asbp_side_scroller_character))

(event `self.ReceiveTick`
  (params (DeltaSeconds :type "Float (single-precision)"))
  (bind (_offset_x _offset_y) (`KismetMathLibrary.BreakVector` (`self.Offset`)))
  (bind _returnvalue_x (`KismetMathLibrary.BreakVector` (`self.K2_GetActorLocation` (`self.Player Reference`))))
  ;[0 1 0.03341 0.5] 2D Camera - Sets location of the Camera with reference from Player Location and Camera Offset
  (bind _result (`/Engine/EditorBlueprintResources/StandardMacros.IncrementFloat` _offset_y)
    (:`  `
      (`self.K2_SetActorLocation` (`KismetMathLibrary.MakeVector` _returnvalue_x _result 600.0)))))

(fn `UserConstructionScript`
  ;[0 1 0.03341 0.5] Comment
  (bind _returnvalue (`GameplayStatics.GetActorOfClass` "/Game/Blueprints/BP_SideScrollerCharacter.BP_SideScrollerCharacter_C"))
  (`self.K2_SetActorLocation` (+ (`self.K2_GetActorLocation` _returnvalue) (`self.Offset`))))