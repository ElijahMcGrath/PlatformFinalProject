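; BP_Gate is an actor, apparently a gate, that moves once when the side-scroller player character hits it.
; The Hit event passes through a DoOnce and a character cast, records the start location, waits a configurable delay, then plays a timeline.
; The timeline alpha drives an eased interpolation from the start to an offset position, set without sweeping.
; The DoOnce precedes the cast, so a first hit by anything else uses up the trigger.
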(event `self.ReceiveHit`
  (params (MyComp :type "PrimitiveComponent Object Reference") (Other :type "Actor Object Reference") (OtherComp :type "PrimitiveComponent Object Reference") (bSelfMoved :type Boolean) (HitLocation :type "Vector Structure") (HitNormal :type "Vector Structure") (NormalImpulse :type "Vector Structure") (Hit :type "HitResult Structure (by ref)"))
  ;[0.05286 1 0 0.502] When Hit player the Gate Moves only Once
  (`/Engine/EditorBlueprintResources/StandardMacros.DoOnce` false
    (:`Completed`
      (cast `/Game/Blueprints/BP_SideScrollerCharacter` Other)
      (set `self.StartingLocation` (`self.K2_GetActorLocation`))
      (`KismetSystemLibrary.Delay` (`self.PlatformIdol`))
      (bind (_direction _alpha) (`Timeline|Timeline` :`NewTime` 2.0)
        (:`Update`
          (`self.K2_SetActorLocation` (`|EaseFunction` (`self.Easing`) _alpha (`self.StartingLocation`) (+ (`self.StartingLocation`) (`self.Offset`)) 2.0 0)))))))

(fn `UserConstructionScript`)