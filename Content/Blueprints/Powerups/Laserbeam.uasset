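; Laserbeam is a powerup projectile actor that damages enemies on contact.
; An actor-level overlap deals fixed damage to BP_Enemy2, while a separate Box component overlap deals the same damage to BP_EnemyBat through EnemyTakeDamage.
; The beam is not destroyed by enemy overlaps, only when a hit involves a WorldStatic component such as a wall.
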(event `self.ReceiveActorBeginOverlap`
  (params (OtherActor :type "Actor Object Reference"))
  ;[1 0 0.2122] Laser deals damage
  (bind _asbp_enemy_2 (cast `/Game/Blueprints/Obstacles/BP_Enemy2` OtherActor))
  (`/Game/Blueprints/Obstacles/BP_Enemy2.Enemy Take damage` _asbp_enemy_2 3))

(event `self.Box.OnComponentBeginOverlap`
  (params (OverlappedComponent :type "PrimitiveComponent Object Reference") (OtherActor :type "Actor Object Reference") (OtherComp :type "PrimitiveComponent Object Reference") (OtherBodyIndex :type Integer) (bFromSweep :type Boolean) (SweepResult :type "HitResult Structure (by ref)"))
  ;[1 0 0.2122] laser deals damage to bat
  (bind _asbp_enemy_bat (cast `/Game/Blueprints/Obstacles/BP_EnemyBat` OtherActor))
  (`/Game/Blueprints/Obstacles/BP_EnemyBat.Enemy Take damage` _asbp_enemy_bat 3))

(event `self.ReceiveHit`
  (params (MyComp :type "PrimitiveComponent Object Reference") (Other :type "Actor Object Reference") (OtherComp :type "PrimitiveComponent Object Reference") (bSelfMoved :type Boolean) (HitLocation :type "Vector Structure") (HitNormal :type "Vector Structure") (NormalImpulse :type "Vector Structure") (Hit :type "HitResult Structure (by ref)"))
  ;[0.05286 1 0 0.502] When Laser hits wall destroy self
  (`/Engine/EditorBlueprintResources/StandardMacros.IsValid` OtherComp
    (:`Is Valid`
      (if (`|EnumEquality` (`PrimitiveComponent.GetCollisionObjectType` OtherComp) "ECC_WorldStatic")
        (`self.K2_DestroyActor`)))))

(fn `UserConstructionScript`)