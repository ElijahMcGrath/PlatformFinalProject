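; Side-scroller bat enemy that drops from the ceiling when the player enters its trigger zone, by enabling physics on its Cube.
; Touching the player damages them through BP_Gameinstance and destroys the bat.
; Hitting a BP_BatFloorTrigger after dropping makes it fire a fan of four BP_BatProjectiles at different pitches and destroy itself.
; Weapon damage reduces its health, and death has a random chance to spawn a heart pickup.
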(event `Enemy Take damage`
  (params (damage :type Integer))
  ;[1 0 0.2122] Enemy takes damage from weapons
  (set `self.Enemy Health` (- (`self.Enemy Health`) damage))
  (if (<= (`self.Enemy Health`) 0)
    (`self.K2_DestroyActor`)
    ;[1 0 0.2122] spawn collectible
    (if (`KismetMathLibrary.RandomBoolWithWeight` 0.3)
      (`|SpawnActorFromClass` "/Game/Blueprints/Powerups/BP_HeartPickup.BP_HeartPickup_C" (`self.GetTransform`) "Undefined" "MultiplyWithRoot" null null))))

(event `self.Box.OnComponentBeginOverlap`
  (params (OverlappedComponent :type "PrimitiveComponent Object Reference") (OtherActor :type "Actor Object Reference") (OtherComp :type "PrimitiveComponent Object Reference") (OtherBodyIndex :type Integer) (bFromSweep :type Boolean) (SweepResult :type "HitResult Structure (by ref)"))
  ;[1 0 0.2122] Player takes damage on overlap
  (if (`self.can take damage again`)
    (cast `/Game/Blueprints/BP_SideScrollerCharacter` OtherActor
      (:`then`
        (bind _asbp_gameinstance (cast `/Game/Blueprints/BP_Gameinstance` (`GameplayStatics.GetGameInstance`)))
        (`/Game/Blueprints/BP_Gameinstance.TakeDamage` _asbp_gameinstance (`self.EnemyAttack`))
        (set `self.can take damage again` false)
        (`self.K2_DestroyActor`))
      (:`CastFailed`
        (cast `/Game/Blueprints/Obstacles/BP_BatFloorTrigger` OtherActor)
        (`self.Enemy hit floor`)))))

(event `Fire Projectiles`
  ;[1 0 0.2122] Explodes when floor collides
  (`|SpawnActorFromClass` "/Game/Blueprints/Obstacles/BP_BatProjectile.BP_BatProjectile_C" (`KismetMathLibrary.MakeTransform` (`SceneComponent.K2_GetComponentLocation` (`self.BatFirepoint`)) (`KismetMathLibrary.MakeRotator` 0.0 10.0)) "AdjustIfPossibleButAlwaysSpawn" "MultiplyWithRoot" null null)
  (`KismetSystemLibrary.PrintString` "ts fired jit")
  (`|SpawnActorFromClass` "/Game/Blueprints/Obstacles/BP_BatProjectile.BP_BatProjectile_C" (`KismetMathLibrary.MakeTransform` (`SceneComponent.K2_GetComponentLocation` (`self.BatFirepoint`)) (`KismetMathLibrary.MakeRotator` 0.0 60.0)) "AdjustIfPossibleButAlwaysSpawn" "MultiplyWithRoot" null null)
  (`KismetSystemLibrary.PrintString` "second")
  (`|SpawnActorFromClass` "/Game/Blueprints/Obstacles/BP_BatProjectile.BP_BatProjectile_C" (`KismetMathLibrary.MakeTransform` (`SceneComponent.K2_GetComponentLocation` (`self.BatFirepoint`)) (`KismetMathLibrary.MakeRotator` 0.0 120.0)) "AdjustIfPossibleButAlwaysSpawn" "MultiplyWithRoot" null null)
  (`KismetSystemLibrary.PrintString` "third")
  (`|SpawnActorFromClass` "/Game/Blueprints/Obstacles/BP_BatProjectile.BP_BatProjectile_C" (`KismetMathLibrary.MakeTransform` (`SceneComponent.K2_GetComponentLocation` (`self.BatFirepoint`)) (`KismetMathLibrary.MakeRotator` 0.0 170.0)) "AdjustIfPossibleButAlwaysSpawn" "MultiplyWithRoot" null null)
  (`KismetSystemLibrary.PrintString` "fourth")
  (`self.K2_DestroyActor`))

(event `self.TriggerZone.OnComponentBeginOverlap`
  (params (OverlappedComponent :type "PrimitiveComponent Object Reference") (OtherActor :type "Actor Object Reference") (OtherComp :type "PrimitiveComponent Object Reference") (OtherBodyIndex :type Integer) (bFromSweep :type Boolean) (SweepResult :type "HitResult Structure (by ref)"))
  ;[1 0 0.2122] Drop from ceilling
  (if (!= true (`self.AlreadyDropped`))
    (cast `/Game/Blueprints/BP_SideScrollerCharacter` OtherActor)
    (set `self.AlreadyDropped` true)
    (`PrimitiveComponent.SetSimulatePhysics` (`self.Cube`) true)))

(event `Enemy hit floor`
  ;[1 0 0.2122] Check if the box has already been dropped, then fire
  (if (`self.AlreadyDropped`)
    (`self.Fire Projectiles`)))

(fn `UserConstructionScript`)