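; BP_Enemy2 is a patrolling obstacle enemy that damages the side-scroller character on overlap.
; After an initial delay, a FlipFlop alternately plays and reverses a Timeline, easing it between its spawn point and an offset in an endless loop.
; Overlap damage goes through BP_Gameinstance.
; EnemyTakedamage reduces health, destroying the enemy at zero with a weighted chance to spawn a BP_HeartPickup.
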(event `self.ReceiveActorBeginOverlap`
  (params (OtherActor :type "Actor Object Reference"))
  ;[1 0 0.2122] Player takes damage on overlap
  (cast `/Game/Blueprints/BP_SideScrollerCharacter` OtherActor)
  (bind _asbp_gameinstance (cast `/Game/Blueprints/BP_Gameinstance` (`GameplayStatics.GetGameInstance`)))
  (`/Game/Blueprints/BP_Gameinstance.TakeDamage` _asbp_gameinstance (`self.EnemyAttack`)))

(event `self.ReceiveBeginPlay`
  ;[0.05286 1 0 0.502] Moves enemy when begin Play
  (set `self.SpawnLocation` (`self.K2_GetActorLocation`))
  (`KismetSystemLibrary.Delay` (`self.EnemyIdol`))
  (`/Engine/EditorBlueprintResources/StandardMacros.FlipFlop` :!label _label
    (:`A`
      (bind (_direction _alpha) (`Timeline|Timeline` :!label _label_2)
        (:`Update`
          (`self.K2_SetActorLocation` (`|EaseFunction` (`self.Easing`) _alpha (`self.SpawnLocation`) (+ (`self.SpawnLocation`) (`self.Offset`)) 2.0 (`self.Steps`))))
        (:`Finished`
          (goto _label))))
    (:`B`
      (goto _label_2 :!via `Reverse`))))

(event `Enemy Take damage`
  (params (damage :type Integer))
  ;[1 0 0.2122] Enemy takes damage from weapons
  (set `self.Enemy Health` (- (`self.Enemy Health`) damage))
  (if (<= (`self.Enemy Health`) 0)
    (`self.K2_DestroyActor`)
    ;[1 0 0.2122] spawn collectible
    (if (`KismetMathLibrary.RandomBoolWithWeight` (`self.CollectibleSpawnChance`))
      (`|SpawnActorFromClass` "/Game/Blueprints/Powerups/BP_HeartPickup.BP_HeartPickup_C" (`self.GetTransform`) "Undefined" "MultiplyWithRoot" null null))))

(fn `UserConstructionScript`)